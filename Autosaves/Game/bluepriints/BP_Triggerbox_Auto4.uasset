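; BP_Triggerbox is a hazard-style trigger that restarts the current level when the player pawn hits its Box component.
; It reacts to a component hit, not an overlap, starts a camera fade-out, waits briefly, then reopens the current level by name.
; The delay is shorter than the fade duration, so the reload begins before the fade completes.
; A reverse fade call is present but unconnected.
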(event OnComponentHit(Box)
  (params (HitComponent :type Primitive%20Component%20Object%20Reference) (OtherActor :type Actor%20Object%20Reference) (OtherComp :type Primitive%20Component%20Object%20Reference) (NormalImpulse :type Vector :default "0, 0, 0") (Hit :type Hit%20Result%20Structure%20%28by%20ref%29))
  (bind _returnvalue (Math|Float|MakeLiteralFloat 2.0))
  (if (== OtherActor (Game|Player|GetPlayerPawn 0))
    (CameraFades|StartCameraFade :self (Game|GetPlayerCameraManager 0) :ToAlpha _returnvalue :Duration _returnvalue)
    (Utilities|FlowControl|Delay 1.0)
    (bind _returnvalue_2 (Game|GetCurrentLevelName true))
    (Game|OpenLevel(byName) (Utilities|String|StringToName _returnvalue_2))))

(fn ConstructionScript)
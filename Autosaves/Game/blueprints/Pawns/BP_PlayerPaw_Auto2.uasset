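; Player pawn for a rolling ball that is driven by torque and restarts the level when it is hit.
; Both movement axes feed one acceleration-mode torque call on X and Y; the TorqueStrengh variable is not applied.
; On Hit, a helper supplies the camera manager and fade time if CanBeDamaged is true, then the camera fades, waits and the current level reopens.
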(event Collision|EventHit
  (params (MyComp :type Primitive%20Component%20Object%20Reference) (Other :type Actor%20Object%20Reference) (OtherComp :type Primitive%20Component%20Object%20Reference) (bSelfMoved :type Boolean) (HitLocation :type Vector :default "0, 0, 0") (HitNormal :type Vector :default "0, 0, 0") (NormalImpulse :type Vector :default "0, 0, 0") (Hit :type Hit%20Result%20Structure%20%28by%20ref%29))
  (bind (_returnvalue _returnvalue2) (CallFunction|NewFunction0))
  (CameraFades|StartCameraFade :self _returnvalue :ToAlpha 1.0 :Duration _returnvalue2)
  (Utilities|FlowControl|Delay _returnvalue2)
  (bind _returnvalue_2 (Game|GetCurrentLevelName true))
  (Game|OpenLevel(byName) (Utilities|String|StringToName _returnvalue_2)))

(event Input|AxisEvents|InputAxisMoveForward/Backward
  (params (AxisValue :type Float%20%28single-precision%29))
  (Class|PrimitiveComponent|AddTorqueinRadians (Variables|Default|GetStaticMeshBall) (Math|Vector|MakeVector (stale Input|AxisEvents|InputAxisMoveLeft/Righ AxisValue) AxisValue 0.0) "None" true))

(event Input|AxisEvents|InputAxisMoveLeft/Righ
  (params (AxisValue :type Float%20%28single-precision%29))
  (Class|PrimitiveComponent|AddTorqueinRadians (Variables|Default|GetStaticMeshBall) (Math|Vector|MakeVector AxisValue (stale Input|AxisEvents|InputAxisMoveForward/Backward AxisValue) 0.0) "None" true))

(fn ConstructionScript)

(fn NewFunction0
  (if (Variables|Actor|GetbCanBeDamaged)
    (return (Game|GetPlayerCameraManager 0) (Math|Float|MakeLiteralFloat 1.0))))
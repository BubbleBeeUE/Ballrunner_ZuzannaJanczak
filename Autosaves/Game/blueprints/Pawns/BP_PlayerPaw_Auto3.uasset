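; Player pawn that rolls a static mesh ball with torque from the move input axes and fades the camera in on BeginPlay.
; Both axes feed one acceleration-change torque call that applies the raw axis value to X and Y alike.
; The ball's hit event is empty, and the TorqueStrengh read and a player-check fade-out with level reload are left unconnected.
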(event OnComponentHit(StaticMeshBall)
  (params (HitComponent :type Primitive%20Component%20Object%20Reference) (OtherActor :type Actor%20Object%20Reference) (OtherComp :type Primitive%20Component%20Object%20Reference) (NormalImpulse :type Vector :default "0, 0, 0") (Hit :type Hit%20Result%20Structure%20%28by%20ref%29)))

(event EventBeginPlay
  (CameraFades|StartCameraFade :self (Game|GetPlayerCameraManager 0) :FromAlpha 1.0 :Duration (Math|Float|MakeLiteralFloat 1.0)))

(event Input|AxisEvents|InputAxisMoveForward/Backward
  (params (AxisValue :type Float%20%28single-precision%29))
  (Class|PrimitiveComponent|AddTorqueinRadians (Variables|Default|GetStaticMeshBall) (Math|Vector|MakeVector (stale Input|AxisEvents|InputAxisMoveLeft/Righ AxisValue) AxisValue 0.0) "None" true))

(event Input|AxisEvents|InputAxisMoveLeft/Righ
  (params (AxisValue :type Float%20%28single-precision%29))
  (Class|PrimitiveComponent|AddTorqueinRadians (Variables|Default|GetStaticMeshBall) (Math|Vector|MakeVector AxisValue (stale Input|AxisEvents|InputAxisMoveForward/Backward AxisValue) 0.0) "None" true))

(fn ConstructionScript)
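; Player pawn for a rolling ball, driven by physics torque from movement input.
; Both movement axes share one AddTorque call that feeds the raw axis value into X and Y as an acceleration change, without a strength multiplier.
; Hit prints a damage message when the pawn can be damaged.
; Unconnected nodes hold a torque-strength copy, camera fades and a level reload, none of which run.
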(event Collision|EventHit
  (params (MyComp :type Primitive%20Component%20Object%20Reference) (Other :type Actor%20Object%20Reference) (OtherComp :type Primitive%20Component%20Object%20Reference) (bSelfMoved :type Boolean) (HitLocation :type Vector :default "0, 0, 0") (HitNormal :type Vector :default "0, 0, 0") (NormalImpulse :type Vector :default "0, 0, 0") (Hit :type Hit%20Result%20Structure%20%28by%20ref%29))
  (if (Variables|Actor|GetbCanBeDamaged)
    (Development|PrintText "Your ball got damaged" true true "(R=0.515625,G=0.086576,B=0.331755,A=1.000000)")))

(event Input|AxisEvents|InputAxisMoveForward/Backward
  (params (AxisValue :type Float%20%28single-precision%29))
  (Class|PrimitiveComponent|AddTorqueinRadians (Variables|Default|GetStaticMeshBall) (Math|Vector|MakeVector (stale Input|AxisEvents|InputAxisMoveLeft/Righ AxisValue) AxisValue 0.0) "None" true))

(event Input|AxisEvents|InputAxisMoveLeft/Righ
  (params (AxisValue :type Float%20%28single-precision%29))
  (Class|PrimitiveComponent|AddTorqueinRadians (Variables|Default|GetStaticMeshBall) (Math|Vector|MakeVector AxisValue (stale Input|AxisEvents|InputAxisMoveForward/Backward AxisValue) 0.0) "None" true))

(fn ConstructionScript)
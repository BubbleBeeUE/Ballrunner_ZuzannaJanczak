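; BP_cristal is a crystal collectable that flies into the player and vanishes when the player overlaps it.
; On overlap, an IsPlayer check gates caching of the start location, actor scale and point light scale, then plays the TL_BlendAlpha timeline.
; Its tracks lerp the crystal toward the player's current position and shrink both crystal and light scale to zero, then the actor is destroyed.
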(event Collision|EventActorBeginOverlap
  (params (OtherActor :type Actor%20Object%20Reference))
  (Utilities|IsPlayer
    (:IsPlayer
      (CallFunction|ActorLocation)
      (CallFunction|ActorSet)
      (bind (_direction _smoothlerpalpha _crack_scale _light) (Timeline|TL_BlendAlpha Play)
        (:Update
          (CallFunction|MoveTowardsActor _smoothlerpalpha)
          (CallFunction|CristalScale _crack_scale)
          (CallFunction|LightAniation _light))
        (:Finished
          (Actor|DestroyActor))))))

(fn ConstructionScript)

(fn MoveTowardsActor
  (params (Alpha :type Float%20%28single-precision%29))
  (Transformation|SetActorLocation (Math|Vector|Lerp(Vector) (Variables|Default|GetLerpStartLocation) (Transformation|GetActorLocation (Game|Player|GetPlayerPawn 0)) Alpha) false false))

(fn ActorLocation
  (Variables|Default|SetLerpStartLocation (Transformation|GetActorLocation)))

(fn CristalScale
  (params (Alpha :type Float%20%28single-precision%29))
  (Transformation|SetActorScale3D (Math|Vector|Lerp(Vector) (Variables|Default|GetCrystalScale) "0, 0, 0" Alpha)))

(fn LightAniation
  (params (Alpha :type Float%20%28single-precision%29))
  (Transformation|SetWorldScale3D (Variables|Default|GetPointLight) (Math|Vector|Lerp(Vector) (Variables|Default|Getlight) "0, 0, 0" Alpha)))

(fn ActorSet
  (Variables|Default|SetCrystalScale (Transformation|GetActorScale3D))
  (Variables|Default|Setlight (Transformation|GetWorldScale (Variables|Default|GetPointLight))))
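; BP_cristal is a collectable crystal that flies to the player and disappears when the player pawn overlaps it.
; On overlap it stores its starting location and plays a timeline that outputs a smoothed alpha.
; Each update lerps from that start to the player's current location, so the crystal homes in on a moving pawn, then destroys itself when the timeline finishes.
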(event Collision|EventActorBeginOverlap
  (params (OtherActor :type Actor%20Object%20Reference))
  (if (== OtherActor (Game|Player|GetPlayerPawn 0))
    (Variables|Default|SetLerpStartLocation (Transformation|GetActorLocation))
    (bind _smoothlerpalpha (Timeline|TL_BlendAlpha Play)
      (:Update
        (CallFunction|MoveTowardsActor _smoothlerpalpha))
      (:Finished
        (Actor|DestroyActor)))))

(fn ConstructionScript)

(fn MoveTowardsActor
  (params (Alpha :type Float%20%28single-precision%29))
  (Transformation|SetActorLocation (Math|Vector|Lerp(Vector) (Variables|Default|GetLerpStartLocation) (Transformation|GetActorLocation (Game|Player|GetPlayerPawn 0)) Alpha) false false))
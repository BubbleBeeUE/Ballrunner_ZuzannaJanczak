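; BP_Cannon_Auto2 is an automatic cannon actor that repeatedly fires BP_Projectale on a timer.
; From BeginPlay it waits the Firerate delay, spawns a projectile at the Arrow component's location and rotation with a configurable Scale, then plays the CannonShoot timeline.
; The timeline animates the Cannon mesh along its local Y axis, and its Finished pin loops back to the delay, so each cycle lasts delay plus animation.
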(event EventBeginPlay
  (Utilities|FlowControl|Delay (Variables|Default|GetFirerate) :!label _label)
  (Game|SpawnActorfromClass "/Game/blueprints/Actors/Projectiles/BP_Projectale.BP_Projectale_C" (Math|Transform|MakeTransform (Transformation|GetWorldLocation (Variables|Default|GetArrow)) (Transformation|GetWorldRotation (Variables|Default|GetArrow)) (Math|Conversions|ToVector(Float) (Variables|Default|Getscale))) "Undefined" 0 0)
  (bind _newtrack_1 (Timeline|CannonShoot PlayFromStart)
    (:Update
      (Transformation|SetRelativeLocation (Variables|Default|Getcannon) (Math|Vector|MakeVector 0.0 _newtrack_1 0.0) false false))
    (:Finished
      (goto _label))))

(fn ConstructionScript)